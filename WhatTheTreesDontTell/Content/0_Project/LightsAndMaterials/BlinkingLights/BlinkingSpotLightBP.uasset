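; Spot light Blueprint that blinks on and off at random intervals during play.
; BeginPlay runs an endless latent loop, alternately hiding and showing the SpotLight, with each Delay drawn from separate off and on random ranges.
; A shared LightBlink function sets the visibility and returns the random wait time.
; The construction script sets whether the BlinkingLightText component is hidden in game through the HideInGame variable.
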(event EventBeginPlay
  (bind _delaytime (CallFunction|LightBlink (Variables|Default|GetLightOffRandRange) true :!label _label))
  (Utilities|FlowControl|Delay _delaytime)
  (bind _delaytime_2 (CallFunction|LightBlink (Variables|Default|GetLightOnRandRange) false))
  (Utilities|FlowControl|Delay _delaytime_2)
  (goto _label))

(fn ConstructionScript
  (Development|SetHiddeninGame (Variables|Default|GetBlinkingLightText) (Variables|Default|GetHideInGame) false))

(fn LightBlink
  (params (RandomRange :type Vector%202D%20Structure) (LightOff :type Boolean))
  (bind (_x _y) (Math|Vector2D|BreakVector2D RandomRange))
  (Development|SetHiddeninGame (Variables|Default|GetSpotLight) LightOff false)
  (return (Math|Random|RandomFloatinRange _x _y)))