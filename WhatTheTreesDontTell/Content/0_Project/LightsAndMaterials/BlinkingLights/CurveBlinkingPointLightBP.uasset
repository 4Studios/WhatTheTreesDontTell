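; Point light Blueprint that blinks following an intensity curve.
; On BeginPlay it caches the light's starting intensity and plays a timeline with its play rate scaled by the blink duration.
; Each timeline update samples the blink curve at the timeline's value and multiplies it by the cached intensity.
; The construction script sets whether the BlinkingLightText label is hidden in game.
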(event EventBeginPlay
  (Variables|Default|SetInitLightIntensity (Variables|/Script/Engine.LightComponentBase|GetIntensity (Variables|Default|GetPointLight)))
  (Components|Timeline|SetPlayRate (Variables|Default|GetBlinkTimeline) (/ 1.0 (Variables|Default|GetBlinkDuration)))
  (bind _blinkcurve (Timeline|BlinkTimeline PlayFromStart)
    (:Update
      (Rendering|Components|Light|SetIntensity (Variables|Default|GetPointLight) (* (Math|Curves|GetFloatValue (Variables|Default|GetBlinkCurve) _blinkcurve) (Variables|Default|GetInitLightIntensity))))))

(fn ConstructionScript
  (Development|SetHiddeninGame (Variables|Default|GetBlinkingLightText) (Variables|Default|GetHideInGame) false))