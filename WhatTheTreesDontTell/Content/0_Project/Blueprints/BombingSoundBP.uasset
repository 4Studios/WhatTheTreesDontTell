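; Bombing sound actor that plays an audible bomb drop followed by its explosion.
; PlayBombingSound starts the FallSound audio component and binds to its finished event.
; When the fall audio ends, it plays ExplosionSound and starts a scaled world-space camera shake on the first player.
; Several disconnected spawn-sound and fade-in nodes remain in the graph unused.
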(event Custom|PlayBombingSound
  (bind _fallsound (Variables|Default|GetFallSound))
  (Audio|Components|Audio|Play _fallsound 0.0)
  (EventDispatchers|AssignOnAudioFinished _fallsound (delegate Custom|OnAudioFallEnd)))

(event Custom|OnAudioFallEnd
  (Audio|Components|Audio|Play (Variables|Default|GetExplosionSound) 0.0)
  (Game|Feedback|ClientStartCameraShake (Game|GetPlayerController 0) "/Game/0_Project/Blueprints/CameraShakeOsBP.CameraShakeOsBP_C" 1.5 "World" "0, 0, 0"))

(fn ConstructionScript)