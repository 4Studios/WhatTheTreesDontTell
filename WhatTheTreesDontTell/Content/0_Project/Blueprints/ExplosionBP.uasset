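; ExplosionBP is an explosion effect actor, fired by its TriggerExplosion event.
; The event optionally shakes the first player's camera, hides the point light, activates its particle system, spawns a scaled-up explosion emitter with sound and fades in fire audio.
; After a short delay, it spawns fire emitters at the locations of the actors in ExtraFireParticles, spreading the aftermath.
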(event Custom|TriggerExplosion
  (params (MakeCameraShake :type Boolean))
  (bind _returnvalue (Transformation|GetActorLocation))
  (if MakeCameraShake
    (Game|Feedback|ClientStartCameraShake (Game|GetPlayerController 0) "/Game/0_Project/Blueprints/CameraShakeOsBP.CameraShakeOsBP_C" 2.0 "CameraLocal" "0, 0, 0"))
  (Rendering|SetVisibility (Variables|Default|GetPointLight) false false)
  (Components|Activation|Activate (Variables|Default|GetParticleSystem) false)
  (Effects|SpawnEmitteratLocation "/Game/StarterContent/Particles/P_Explosion.P_Explosion" _returnvalue "0, 0, 0" "3.000000,3.000000,3.000000")
  (Audio|PlaySoundatLocation "/Game/StarterContent/Audio/Explosion01.Explosion01" _returnvalue "0, 0, 0" 1.0 1.0 0.0 0 0 0)
  (Audio|Components|Audio|FadeIn (Variables|Default|GetFireSound) 2.0 1.0 0.0 "Logarithmic" :!class /Script/Engine.AudioComponent)
  (Utilities|FlowControl|Delay 2.0)
  (for _array_element (Variables|Default|GetExtraFireParticles)
    (Effects|SpawnEmitteratLocation "/Game/StarterContent/Particles/P_Fire.P_Fire" (Transformation|GetActorLocation _array_element))))

(fn ConstructionScript)