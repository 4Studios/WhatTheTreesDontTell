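; Generic box trigger actor that fires the TriggerActivation dispatcher when an overlapping actor carries any of its ActivationTags.
; Overlaps count only while Activated, which other Blueprints toggle through EnableTrigger and DisableTrigger.
; An optional DoOnce setting limits firing to once until ResetDoOnce is called, and each activation prints a debug string.
; The construction script applies box size, displayed text and in-game visibility from variables.
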(event OnComponentBeginOverlap(Collider)
  (params (OverlappedComponent :type Primitive%20Component%20Object%20Reference) (OtherActor :type Actor%20Object%20Reference) (OtherComp :type Primitive%20Component%20Object%20Reference) (OtherBodyIndex :type Integer) (bFromSweep :type Boolean) (SweepResult :type Hit%20Result%20Structure%20%28by%20ref%29))
  (if (Variables|Default|GetActivated)
    ;[0.4646 1 0.669] Check Activation Tags
    (Variables|Default|SetActivateTrigger false)
    (for _array_element (Variables|Default|GetActivationTags)
      (if (Actor|ActorHasTag OtherActor _array_element)
        (Variables|Default|SetActivateTrigger true)))
    ;[0.4999 1 0.5472] Activate Trigger
    (if (Variables|Default|GetActivateTrigger)
      (if (Variables|Default|GetDoOnce)
        (Utilities|FlowControl|DoOnce false
          (:Completed
            _)))
      (Default|CallTriggerActivationDispatcher)
      (Development|PrintString "ENTERED TRIGGER" true true "(R=0.000000,G=0.721569,B=1.000000,A=1.000000)"))))

(event Custom|ResetDoOnce
  ;[1 0.4547 0.8778] Externally Reset DoOnce
  ;[0.4999 1 0.5472] Activate Trigger
  (Utilities|FlowControl|DoOnce false) ; enters at Reset
)

(event Custom|EnableTrigger
  ;[0.5434 0.5798 1] Enable/Disable Trigger from other BP
  (Variables|Default|SetActivated true))

(event Custom|DisableTrigger
  ;[0.5434 0.5798 1] Enable/Disable Trigger from other BP
  (Variables|Default|SetActivated false))

(fn ConstructionScript
  (Components|Box|SetBoxExtent (Variables|Default|GetCollider) (Variables|Default|GetTriggerSize) true)
  (Rendering|Components|TextRender|SetText (Variables|Default|GetText) (Variables|Default|GetTextDisplayed))
  (Rendering|SetActorHiddenInGame (Variables|Default|GetHiddenInGame)))