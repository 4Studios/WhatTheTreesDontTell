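; Trigger volume that repeatedly damages the player while they stand inside it.
; On overlap by a Player-tagged actor it damages the FPSCharNew player, then loops after a random delay between MinDelay and MaxDelay until the player leaves.
; The construction script sizes the box collider from TriggerSize and sets its in-game visibility from HideInGame.
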(event OnComponentBeginOverlap(Collider)
  (params (OverlappedComponent :type Primitive%20Component%20Object%20Reference) (OtherActor :type Actor%20Object%20Reference) (OtherComp :type Primitive%20Component%20Object%20Reference) (OtherBodyIndex :type Integer) (bFromSweep :type Boolean) (SweepResult :type Hit%20Result%20Structure%20%28by%20ref%29))
  (if (Actor|ActorHasTag OtherActor "Player")
    (Variables|Default|SetPlayerInside true)
    (Default|ApplyDamage (.AsFPSChar%20New (Utilities|Casting|CastToFPSCharNew (Game|GetPlayerCharacter 0))) (Variables|Default|GetDamageAmount) (Transformation|GetActorLocation) false :!label _label)
    (Utilities|FlowControl|Delay (Math|Random|RandomFloatinRange (Variables|Default|GetMinDelay) (Variables|Default|GetMaxDelay)))
    (if (Variables|Default|GetPlayerInside)
      (goto _label))))

(event OnComponentEndOverlap(Collider)
  (params (OverlappedComponent :type Primitive%20Component%20Object%20Reference) (OtherActor :type Actor%20Object%20Reference) (OtherComp :type Primitive%20Component%20Object%20Reference) (OtherBodyIndex :type Integer))
  (if (Actor|ActorHasTag OtherActor "Player")
    (Variables|Default|SetPlayerInside false)))

(fn ConstructionScript
  (Components|Box|SetBoxExtent (Variables|Default|GetCollider) (Variables|Default|GetTriggerSize) true)
  (Development|SetHiddeninGame (Variables|Default|GetCollider) (Variables|Default|GetHideInGame) false))