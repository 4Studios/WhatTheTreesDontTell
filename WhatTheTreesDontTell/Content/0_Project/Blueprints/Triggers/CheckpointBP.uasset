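; Checkpoint trigger with a configurable box collider that saves the player's progress the first time a tagged Player overlaps it while Activated.
; The overlap loads or creates the "SaveGame" slot, then stores the level-plus-checkpoint name and actor reference in SaveGameBP.
; ActivateCheckpoint, also gated by Activated, disables collision, fires a dispatcher and recursively calls itself on PrevCheckpoint, propagating back along the checkpoint chain.
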(event OnComponentBeginOverlap(Collider)
  (params (OverlappedComponent :type Primitive%20Component%20Object%20Reference) (OtherActor :type Actor%20Object%20Reference) (OtherComp :type Primitive%20Component%20Object%20Reference) (OtherBodyIndex :type Integer) (bFromSweep :type Boolean) (SweepResult :type Hit%20Result%20Structure%20%28by%20ref%29))
  (if (and (Variables|Default|GetActivated) (Actor|ActorHasTag OtherActor "Player"))
    (Utilities|FlowControl|DoOnce false
      (:Completed
        (Development|PrintString "ENTERED CHECKPOINT" true true "(R=0.068719,G=1.000000,B=0.000000,A=1.000000)")
        (bind _returnvalue (SaveGame|DoesSaveGameExist "SaveGame"))
        (if _returnvalue
          (bind _returnvalue_2 (SaveGame|LoadGamefromSlot "SaveGame"))
          (Variables|Default|SetSaveGame _returnvalue_2)
          (else
            (bind _returnvalue_3 (SaveGame|CreateSaveGameObject "/Game/0_Project/Blueprints/Game/SaveGameBP.SaveGameBP_C"))
            (Variables|Default|SetSaveGame _returnvalue_3)))
        (bind _returnvalue_4 (Game|GetCurrentLevelName true))
        (Variables|/Game/0_Project/Blueprints/Game/SaveGameBP.SaveGameBP_C|SetLastCheckpointName (.AsSave%20Game%20BP (Utilities|Casting|CastToSaveGameBP (Variables|Default|GetSaveGame))) (Utilities|String|Append _returnvalue_4 "___" (Utilities|GetDisplayName self)))
        (Variables|/Game/0_Project/Blueprints/Game/SaveGameBP.SaveGameBP_C|SetLastCheckpointActor (.AsSave%20Game%20BP (Utilities|Casting|CastToSaveGameBP (Variables|Default|GetSaveGame))) self)
        (SaveGame|SaveGametoSlot (Variables|Default|GetSaveGame) "SaveGame")
        (Development|PrintString "SAVED CHECKPOINT" true true "(R=0.068719,G=1.000000,B=0.000000,A=1.000000)")))))

(event Custom|ActivateCheckpoint
  (bind _prevcheckpoint (Variables|Default|GetPrevCheckpoint))
  (if (Variables|Default|GetActivated)
    (Development|PrintString "CHECKPOINT TRIGGERED" true true "(R=0.068719,G=1.000000,B=0.000000,A=1.000000)")
    (Collision|SetActorEnableCollision false)
    (Default|CallCheckpointActivateDispatcher)
    (Utilities|IsValid _prevcheckpoint
      (:Is%20Valid
        (CallFunction|ActivateCheckpoint _prevcheckpoint)))))

(fn ConstructionScript
  (bind _collider (Variables|Default|GetCollider))
  (Development|SetHiddeninGame _collider (Variables|Default|GetHideInGame) true)
  (Components|Box|SetBoxExtent _collider (Variables|Default|GetCheckpointSize) true))