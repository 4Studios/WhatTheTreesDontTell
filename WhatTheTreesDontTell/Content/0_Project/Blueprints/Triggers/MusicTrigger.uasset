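; MusicTrigger is a box trigger volume that plays a configurable music track while an actor tagged Player is inside.
; Entry activates and plays the audio component; exit fades it out, then stops and deactivates it after an uncancelled delay matching the fade.
; The construction script applies the box size and sound, and sets collider visibility from HideInGame and a packaged-for-distribution check.
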(event OnComponentBeginOverlap(Collider)
  (params (OverlappedComponent :type Primitive%20Component%20Object%20Reference) (OtherActor :type Actor%20Object%20Reference) (OtherComp :type Primitive%20Component%20Object%20Reference) (OtherBodyIndex :type Integer) (bFromSweep :type Boolean) (SweepResult :type Hit%20Result%20Structure%20%28by%20ref%29))
  (bind _audiocomp (Variables|Default|GetAudioComp))
  (if (Actor|ActorHasTag OtherActor "Player")
    (Components|Activation|SetActive _audiocomp true false)
    (Audio|Components|Audio|Play _audiocomp 0.0)))

(event OnComponentEndOverlap(Collider)
  (params (OverlappedComponent :type Primitive%20Component%20Object%20Reference) (OtherActor :type Actor%20Object%20Reference) (OtherComp :type Primitive%20Component%20Object%20Reference) (OtherBodyIndex :type Integer))
  (bind _audiocomp (Variables|Default|GetAudioComp))
  (if (Actor|ActorHasTag OtherActor "Player")
    (Audio|Components|Audio|FadeOut _audiocomp 2.0 0.0 "SCurve" :!class /Script/Engine.AudioComponent)
    (Utilities|FlowControl|Delay 2.0)
    (Audio|Components|Audio|Stop _audiocomp)
    (Components|Activation|SetActive _audiocomp false false)))

(fn ConstructionScript
  (Components|Box|SetBoxExtent (Variables|Default|GetCollider) (Variables|Default|GetTriggerSize) true)
  (Development|SetHiddeninGame (Variables|Default|GetCollider) (and (Variables|Default|GetHideInGame) (not (Class|KismetSystemLibrary|IsPackagedforDistribution))) true)
  (Audio|Components|Audio|SetSound (Variables|Default|GetAudioComp) (Variables|Default|GetMusicToPlay)))