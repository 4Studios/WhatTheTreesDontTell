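; Trigger volume that fires a dispatcher when the player camera looks at its linked LookAtProbe actor.
; While activated, overlaps by actors with matching ActivationTags toggle Tick, which line-traces along camera forward on the Camera channel.
; A probe hit calls the dispatcher every tick, or once until externally reset if DoOnce is set.
; The construction script applies box size, label, visibility and probe radius; other Blueprints can enable or disable it.
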(event OnComponentBeginOverlap(Collider)
  (params (OverlappedComponent :type Primitive%20Component%20Object%20Reference) (OtherActor :type Actor%20Object%20Reference) (OtherComp :type Primitive%20Component%20Object%20Reference) (OtherBodyIndex :type Integer) (bFromSweep :type Boolean) (SweepResult :type Hit%20Result%20Structure%20%28by%20ref%29))
  (if (Variables|Default|GetActivated)
    ;[0.4646 1 0.669] Check Activation Tags On Begin Overlap
    (Variables|Default|SetActivateTrigger false)
    (for _array_element (Variables|Default|GetActivationTags)
      (if (Actor|ActorHasTag OtherActor _array_element)
        (Variables|Default|SetActivateTrigger true)))
    ;[0.4999 1 0.5472] Activate Tick
    (if (Variables|Default|GetActivateTrigger)
      (Actor|Tick|SetActorTickEnabled true)
      (Development|PrintString "ENTERED ON LOOKAT TRIGGER" true true "(R=0.000000,G=0.721569,B=1.000000,A=1.000000)"))))

(event OnComponentEndOverlap(Collider)
  (params (OverlappedComponent :type Primitive%20Component%20Object%20Reference) (OtherActor :type Actor%20Object%20Reference) (OtherComp :type Primitive%20Component%20Object%20Reference) (OtherBodyIndex :type Integer))
  (if (Variables|Default|GetActivated)
    ;[1 0.9408 0.3957] Check Activation Tags On End Overlap
    (Variables|Default|SetActivateTrigger false)
    (for _array_element (Variables|Default|GetActivationTags)
      (if (Actor|ActorHasTag OtherActor _array_element)
        (Variables|Default|SetActivateTrigger true)))
    ;[1 0.9408 0.3957] Deactivate Tick
    (if (Variables|Default|GetActivateTrigger)
      (Actor|Tick|SetActorTickEnabled false)
      (Development|PrintString "EXITED LOOKAT TRIGGER" true true "(R=0.000000,G=0.721569,B=1.000000,A=1.000000)"))))

(event Custom|ResetDoOnce
  ;[1 0.4547 0.8778] Externally Reset DoOnce
  ;[1 0.6273 0.2193] Check for Visibility Hit & DoOnce
  (Utilities|FlowControl|DoOnce false) ; enters at Reset
)

(event Custom|EnableTrigger
  ;[0.5434 0.5798 1] Enable/Disable Trigger from other BP
  (Variables|Default|SetActivated true))

(event Custom|DisableTrigger
  ;[0.5434 0.5798 1] Enable/Disable Trigger from other BP
  (Variables|Default|SetActivated false))

(event Custom|ResetLookingPrint
  ;[1 0.6273 0.2193] Check for Visibility Hit & DoOnce
  (Utilities|FlowControl|DoOnce false) ; enters at Reset
)

(event Custom|ResetNotLookingPrint
  (Utilities|FlowControl|DoOnce false) ; enters at Reset
)

(event EventTick
  (params (DeltaSeconds :type Float%20%28single-precision%29))
  (bind _returnvalue (Game|GetPlayerCameraManager 0))
  (bind _returnvalue_2 (Camera|GetCameraLocation _returnvalue))
  ;[0 0.9213 1] On Tick Enabled, RayCast
  (bind (_outhit _returnvalue_3) (Collision|LineTraceByChannel _returnvalue_2 (+ _returnvalue_2 (* (Transformation|GetActorForwardVector _returnvalue) 5.12e+04)) "TraceTypeQuery2" true 0 "None" true "(R=1.000000,G=0.000000,B=0.000000,A=1.000000)" "(R=0.000000,G=1.000000,B=0.000000,A=1.000000)" 1.0))
  ;[1 0.6273 0.2193] Check for Visibility Hit & DoOnce
  (if _returnvalue_3
    (if (== (.HitActor (Collision|BreakHitResult _outhit)) (Variables|Default|GetLookAtProbe))
      (if (Variables|Default|GetDoOnce)
        (Utilities|FlowControl|DoOnce false
          (:Completed
            _)))
      (Default|CallLookatDispatcher)
      (Utilities|FlowControl|DoOnce false
        (:Completed
          (Development|PrintString "LookingAt Probe" true true "(R=0.000000,G=0.203922,B=1.000000,A=1.000000)")
          (CallFunction|ResetNotLookingPrint)))
      (else
        (Utilities|FlowControl|DoOnce false :!label _label
          (:Completed
            (Development|PrintString "Not LookingAt Probe" true true "(R=0.000000,G=0.203922,B=1.000000,A=1.000000)")
            (CallFunction|ResetLookingPrint)))))
    (else
      (goto _label))))

(fn ConstructionScript
  (bind _hiddeningame (Variables|Default|GetHiddenInGame))
  (bind _lookatprobe (Variables|Default|GetLookAtProbe))
  (Components|Box|SetBoxExtent (Variables|Default|GetCollider) (Variables|Default|GetTriggerSize) true)
  (Rendering|Components|TextRender|SetText (Variables|Default|GetText) (Variables|Default|GetTextDisplayed))
  (Rendering|SetActorHiddenInGame _hiddeningame)
  (Rendering|SetActorHiddenInGame _lookatprobe _hiddeningame)
  (Components|Sphere|SetSphereRadius (Variables|/Game/0_Project/Blueprints/Triggers/LookAtTrigger_Probe.LookAtTrigger_Probe_C|GetLookAtSphere _lookatprobe) (Variables|Default|GetProbeRadius) true))