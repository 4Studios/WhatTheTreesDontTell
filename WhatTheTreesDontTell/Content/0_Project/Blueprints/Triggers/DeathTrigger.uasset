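; DeathTrigger is a box volume that kills the player on contact.
; When an actor tagged Player begins overlapping the Collider, it calls PlayerDeath on the FPSCharacter of player 0.
; The construction script sizes the box from TriggerSize and sets its in-game visibility from HideInGame.
; A DoOnce node is left in the graph but never runs, so the trigger can fire repeatedly.
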(event OnComponentBeginOverlap(Collider)
  (params (OverlappedComponent :type Primitive%20Component%20Object%20Reference) (OtherActor :type Actor%20Object%20Reference) (OtherComp :type Primitive%20Component%20Object%20Reference) (OtherBodyIndex :type Integer) (bFromSweep :type Boolean) (SweepResult :type Hit%20Result%20Structure%20%28by%20ref%29))
  (if (Actor|ActorHasTag OtherActor "Player")
    (Default|PlayerDeath (.AsFPSCharacter (Utilities|Casting|CastToFPSCharacter (Game|GetPlayerCharacter 0))) true)))

(fn ConstructionScript
  (Components|Box|SetBoxExtent (Variables|Default|GetCollider) (Variables|Default|GetTriggerSize) true)
  (Development|SetHiddeninGame (Variables|Default|GetCollider) (Variables|Default|GetHideInGame) true))