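; Helicopter actor for intro and outro cutscenes, flying away on take-off and later returning to land.
; Chained timelines lerp the pivot's location and rotation between placed waypoint actors through a shared MoveHelicopter event.
; Take-off ends by fading out sound and hiding the helicopter; landing reveals it, fades sound in, then ping-pongs an idle timeline.
; Tick continuously spins the top and rear rotors.
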(event Custom|TriggerHelicopterTakeOff
  ;[0.6868 0.9801 1] Intro Animation
  (bind _takeofftrack (Timeline|TakeOffTimeline PlayFromStart)
    (:Update
      (CallFunction|MoveHelicopter (Variables|Default|GetInitialPosition) (Variables|Default|GetSecondPosition) _takeofftrack))
    (:Finished
      (bind _leavetrack (Timeline|LeaveTimeline PlayFromStart)
        (:Update
          (CallFunction|MoveHelicopter (Variables|Default|GetSecondPosition) (Variables|Default|GetThirdPosition) _leavetrack))
        (:Finished
          (Audio|Components|Audio|FadeOut (Variables|Default|GetHelicopterSound) 5.0 0.0 "Logarithmic" :!class /Script/Engine.AudioComponent)
          (Development|SetHiddeninGame (Variables|Default|GetHelicopterPivotRoot) true true))))))

(event Custom|MoveHelicopter
  (params (InitialTransform :type Actor%20Object%20Reference) (FinalTransform :type Actor%20Object%20Reference) (CurrentMovementTime :type Float%20%28single-precision%29))
  (bind _helicopterpivotroot (Variables|Default|GetHelicopterPivotRoot))
  ;[0.7243 1 0.5684] HelicopterMovement
  (Transformation|SetWorldLocation _helicopterpivotroot (Math|Vector|Lerp(Vector) (Transformation|GetActorLocation InitialTransform) (Transformation|GetActorLocation FinalTransform) CurrentMovementTime) false false)
  (Transformation|SetRelativeRotation _helicopterpivotroot (Math|Rotator|Lerp(Rotator) (Transformation|GetActorRotation InitialTransform) (Transformation|GetActorRotation FinalTransform) CurrentMovementTime true) false false))

(event Custom|TriggerHelicopterLanding
  (bind _helicoptersound (Variables|Default|GetHelicopterSound))
  ;[0.6868 0.9801 1] Outro Animation
  (Audio|Components|Audio|FadeIn _helicoptersound 0.1 0.5 0.0 "Logarithmic" :!class /Script/Engine.AudioComponent)
  (Audio|Components|Audio|FadeIn _helicoptersound 5.0 4.0 0.0 "Linear" :!class /Script/Engine.AudioComponent)
  (Development|SetHiddeninGame (Variables|Default|GetHelicopterPivotRoot) false true)
  (bind _leavetrack (Timeline|ReturningTimeline PlayFromStart)
    (:Update
      (CallFunction|MoveHelicopter (Variables|Default|GetReturningInitialPosition) (Variables|Default|GetReturningFinalPosition) _leavetrack))
    (:Finished
      (bind _takeofftrack (Timeline|LandingTimeline PlayFromStart)
        (:Update
          (CallFunction|MoveHelicopter (Variables|Default|GetReturningFinalPosition) (Variables|Default|GetLandingPosition) _takeofftrack))
        (:Finished
          (bind (_direction _timetrack) (Timeline|IdleHoldTimeline Play)
            (:Update
              (CallFunction|MoveHelicopter (Variables|Default|GetLandingPosition) (Variables|Default|GetIdlePosition) _timetrack))
            (:Finished
              (Utilities|FlowControl|Delay 0.01)
              (switch Utilities|FlowControl|Switch|SwitchonETimelineDirection _direction
                (:Forward
                  (Timeline|IdleHoldTimeline ReverseFromEnd))
                (:Backward
                  (Timeline|IdleHoldTimeline PlayFromStart))))))))))

(event EventTick
  (params (DeltaSeconds :type Float%20%28single-precision%29))
  (bind _helixrotationspeed (Variables|Default|GetHelixRotationSpeed))
  (bind _returnvalue (* DeltaSeconds _helixrotationspeed))
  ;[0.9936 0.655 1] Helicopter Rotors Rotation
  (Transformation|AddLocalRotation (Variables|Default|GetRepivotTopRotor) (Math|Rotator|MakeRotator 0.0 0.0 _returnvalue) false false)
  (Transformation|AddLocalRotation (Variables|Default|GetRepivotRearRotor) (Math|Rotator|MakeRotator _returnvalue 0.0 0.0) false false))

(fn ConstructionScript)